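; Turret projectile actor that damages the GLaDOS player pawn on contact.
; Tick moves it in a straight line by Speed and Direction without sweeping.
; Its Box overlap casts to BP_GladosPawn, calls DamageGlados and destroys the bullet; other actors are ignored.
; Target-seeking logic is left disconnected, so nothing in this file sets Direction at runtime.
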(event OnComponentBeginOverlap(Box)
  (params (OverlappedComponent :type Primitive%20Component%20Object%20Reference) (OtherActor :type Actor%20Object%20Reference) (OtherComp :type Primitive%20Component%20Object%20Reference) (OtherBodyIndex :type Integer) (bFromSweep :type Boolean) (SweepResult :type Hit%20Result%20Structure%20%28by%20ref%29))
  (bind _asbp_glados_pawn (Utilities|Casting|CastToBP_GladosPawn OtherActor))
  (Default|DamageGlados _asbp_glados_pawn)
  (Actor|DestroyActor))

(event EventBeginPlay)

(event Collision|EventActorBeginOverlap
  (params (OtherActor :type Actor%20Object%20Reference)))

(event EventTick
  (params (DeltaSeconds :type Float%20%28single-precision%29))
  (Transformation|SetActorLocation (+ (Transformation|GetActorLocation) (* DeltaSeconds (* (Variables|Default|GetSpeed) (Variables|Default|GetDirection)))) false false))

(fn ConstructionScript)

(fn FindTargetDirection)