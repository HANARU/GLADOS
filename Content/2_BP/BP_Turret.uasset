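; Turret that aims a red laser beam at the player when its PawnSensing component sees them; it has no firing or damage logic.
; Each sighting rotates LaserPoint toward the player horizontally by zeroing both Z values, then runs LaserTrack.
; LaserTrack line-traces forward and, on a blocking hit, shows the laser effect ending at the impact point.
; The laser starts hidden and is never hidden again once shown.
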(event OnSeePawn(PawnSensing)
  (params (Pawn :type Pawn%20Object%20Reference))
  (bind _returnvalue (Game|GetPlayerCharacter 0))
  (bind _laserpoint (Variables|Default|GetLaserPoint))
  (bind _returnvalue_2 (Transformation|GetWorldLocation _laserpoint))
  (if (== Pawn _returnvalue)
    (bind _asbp_single_player (Utilities|Casting|CastToBP_SinglePlayer _returnvalue))
    (bind _output_get (Variables|Default|SetWatchingRotation (Math|Rotator|FindLookatRotation (Math|Vector|MakeVector (.x _returnvalue_2) (.y _returnvalue_2) 0.0) (Math|Vector|MakeVector (.x (Transformation|GetActorLocation _asbp_single_player)) (.y (Transformation|GetActorLocation _asbp_single_player)) 0.0))))
    (Transformation|SetWorldRotation (Variables|Default|GetLaserPoint) _output_get false false)
    (CallFunction|LaserTrack)))

(event Custom|LaserTrack
  (bind _laserpoint (Variables|Default|GetLaserPoint))
  (bind _laser (Variables|Default|GetLaser))
  (bind _returnvalue (Transformation|GetWorldLocation _laserpoint))
  (bind _output_get (Variables|Default|SetEndVector (+ _returnvalue (* (Math|Vector|GetForwardVector _laserpoint) (Variables|Default|GetDistance)))))
  (bind _outhit (Collision|LineTraceByChannel _returnvalue _output_get "TraceTypeQuery6" false 0 "None" true "(R=1.000000,G=1.000000,B=0.000000,A=1.000000)" "(R=1.000000,G=0.076232,B=0.000000,A=1.000000)"))
  (bind _output_get_2 (Variables|Default|SetHit%20Bool (.bBlockingHit (Collision|BreakHitResult _outhit))))
  (if _output_get_2
    (Rendering|SetVisibility _laser true false)
    (bind _output_get_3 (Variables|Default|SetHit%20Location (.Location (Collision|BreakHitResult _outhit))))
    (Effects|Components|ParticleSystem|SetVectorParameter _laser "LaserEnd" _output_get_3)))

(event EventBeginPlay
  (bind _laser (Variables|Default|GetLaser))
  (Rendering|SetVisibility _laser false false)
  (Effects|Components|ParticleSystem|SetColorParameter _laser "Color" "(R=1.000000,G=0.008924,B=0.000000,A=1.000000)")
  (Effects|Components|ParticleSystem|SetFloatParameter _laser "LaserWidth" 1.0))

(fn ConstructionScript)