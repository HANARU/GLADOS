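; GLaDOS boss pawn that takes missile hits and plays a death sequence.
; Each DamageGlados call spawns an explosion, and a MultiGate destroys one cube per hit for three hits, spawning a BP_GlaDosBall in its place.
; The fourth hit starts DestroyBoss, an endless delayed loop of randomly offset explosions and camera shake.
; Tick shows the BP_BossKill widget once the explosion counter passes its threshold.
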(event Custom|DamageGlados
  (params (Missle :type BP%20Turret%20Missle%20Object%20Reference))
  (bind _returnvalue (Transformation|GetActorTransform Missle))
  (Effects|SpawnEmitteratLocation "/Game/3_Assets/FX/Particles/P_ky_explosion.P_ky_explosion" (.location _returnvalue) (.rotation _returnvalue))
  (Utilities|FlowControl|MultiGate false false 0
    (:Out%200
      (CallFunction|DestroyComponent (Variables|Default|GetCube)))
    (:Out%201
      (CallFunction|DestroyComponent (Variables|Default|GetCube1)))
    (:Out%202
      (CallFunction|DestroyComponent (Variables|Default|GetCube2)))
    (:Out%203
      (CallFunction|DestroyBoss))))

(event Custom|DestroyBoss
  (for _array_element (Variables|Default|GetRandomLocation) :!label _label
    (Effects|SpawnEmitteratLocation "/Game/3_Assets/FX/Particles/P_ky_hit1.P_ky_hit1" (+ _array_element (+ (Math|Vector|MakeVector (Math|Random|RandomFloatinRange (Variables|Default|GetMin) (Variables|Default|GetMax)) (Math|Random|RandomFloatinRange (Variables|Default|GetMin) (Variables|Default|GetMax)) (Math|Random|RandomFloatinRange (Variables|Default|GetMin) (Variables|Default|GetMax))) (Transformation|GetActorLocation))))
    (Math|Integer|IncrementInt (Variables|Default|GetExplosionTime)))
  (bind _asbp_single_player (Utilities|Casting|CastToBP_SinglePlayer (Game|GetPlayerCharacter 0)))
  (Camera|PlayWorldCameraShake "/Game/2_BP/BP_CameraShake.BP_CameraShake_C" (Transformation|GetWorldLocation (Variables|/Script/GLADOS.SinglePlayer|GetFPSCAM _asbp_single_player)) 0.0 5e+02)
  (Utilities|FlowControl|Delay 0.5)
  (goto _label))

(event Collision|EventActorBeginOverlap
  (params (OtherActor :type Actor%20Object%20Reference)))

(event EventTick
  (params (DeltaSeconds :type Float%20%28single-precision%29))
  (if (> (Variables|Default|GetExplosionTime) 30)
    (Utilities|FlowControl|DoOnce false
      (:Completed
        (bind _returnvalue (UserInterface|CreateWidget "/Game/2_BP/BP_UI/BP_BossKill.BP_BossKill_C"))
        (UserInterface|Viewport|AddtoViewport _returnvalue 0)))))

(fn ConstructionScript)

(fn DestroyComponent
  (params (Component :type Static%20Mesh%20Component%20Object%20Reference))
  (Utilities|IsValid Component
    (:Is%20Valid
      (bind _output_get (Variables|Default|SetCubeLocation (Transformation|GetWorldLocation Component)))
      (Components|DestroyComponent Component)
      (Game|SpawnActorfromClass "/Game/2_BP/BP_GlaDosBall.BP_GlaDosBall_C" (Math|Transform|MakeTransform _output_get "0, 0, 0" "1.000000,1.000000,1.000000") "Undefined" "MultiplyWithRoot" 0 0))))