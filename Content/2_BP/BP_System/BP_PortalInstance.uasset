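; BP_PortalInstance, likely the game instance, manages the intro and main menu screens and stops sound cues.
; IntroVideo and ShowMainMenu lazily create and cache their widgets, add them to the viewport and switch to UI-only input.
; The intro hides the mouse cursor, while the menu shows it and plays its music as 2D sound.
; StopAllSound stops four stored cues, which do not include the menu music.
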(event Custom|IntroVideo
  (bind _returnvalue (Game|GetPlayerController 0))
  (Utilities|IsValid (Variables|Default|GetIntro)
    (:Is%20Valid
      _)
    (:Is%20Not%20Valid
      (bind _returnvalue_2 (UserInterface|CreateWidget "/Game/2_BP/BP_UI/UI_Intro.UI_Intro_C"))
      (bind _output_get (Variables|Default|SetIntro _returnvalue_2))))
  (UserInterface|Viewport|AddtoViewport _output_get 0)
  (Input|SetInputModeUIOnly _returnvalue _output_get "DoNotLock" false)
  (Variables|/Script/Engine.PlayerController|SetbShowMouseCursor _returnvalue false))

(event Custom|ShowMainMenu
  (bind _returnvalue (Game|GetPlayerController 0))
  (Utilities|IsValid (Variables|Default|GetMainMenu)
    (:Is%20Valid
      _)
    (:Is%20Not%20Valid
      (bind _returnvalue_2 (UserInterface|CreateWidget "/Game/2_BP/BP_UI/UI_MainMenu.UI_MainMenu_C"))
      (bind _output_get (Variables|Default|SetMainMenu _returnvalue_2))))
  (UserInterface|Viewport|AddtoViewport _output_get 0)
  (Input|SetInputModeUIOnly _returnvalue _output_get "DoNotLock" false)
  (Variables|/Script/Engine.PlayerController|SetbShowMouseCursor _returnvalue true)
  (Audio|PlaySound2D "/Game/3_Assets/1_MainMenu/BGM_MainMenu.BGM_MainMenu" 1.0 1.0 0.0 0 0))

(event Custom|Stop%20All%20Sound
  (Audio|Components|Audio|Stop (Variables|Default|GetCue_1st)))