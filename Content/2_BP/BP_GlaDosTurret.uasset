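; GLaDOS turret actor that faces the player and fires bullets on a repeating timer.
; Tick spawns a BP_GlaDosTurretBullet at the Arrow every SpawnTime, whether or not the player is seen.
; PawnSensing turns the actor toward the player on yaw only, then runs a Visibility line trace from the Arrow.
; A blocking hit shows the Laser effect ending at the impact point; nothing hides it again after BeginPlay.
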(event OnSeePawn(PawnSensing)
  (params (Pawn :type Pawn%20Object%20Reference))
  (bind _returnvalue (Game|GetPlayerCharacter 0))
  (bind _returnvalue_2 (Transformation|GetActorLocation))
  ;[1 1 1] 플레이어 추적
  (if (== Pawn _returnvalue)
    (bind _asbp_single_player (Utilities|Casting|CastToBP_SinglePlayer _returnvalue))
    (bind _output_get (Variables|Default|SetWahchingRotation (Math|Rotator|FindLookatRotation (Math|Vector|MakeVector (.x _returnvalue_2) (.y _returnvalue_2) 0.0) (Math|Vector|MakeVector (.x (Transformation|GetActorLocation _asbp_single_player)) (.y (Transformation|GetActorLocation _asbp_single_player)) 0.0))))
    (Transformation|SetActorRotation _output_get)
    (CallFunction|LaserTrack)))

(event Custom|LaserTrack
  (bind _arrow (Variables|Default|GetArrow))
  (bind _laser (Variables|Default|GetLaser))
  (bind _returnvalue (Transformation|GetWorldLocation _arrow))
  ;[1 1 1] 레이저
  (bind _output_get (Variables|Default|SetEndVector (* _returnvalue (* (Math|Vector|GetForwardVector _arrow) (Variables|Default|GetDistance)))))
  (bind _outhit (Collision|LineTraceByChannel _returnvalue _output_get "TraceTypeQuery1" false 0 "None"))
  (bind _output_get_2 (Variables|Default|SetHitBool (.bBlockingHit (Collision|BreakHitResult _outhit))))
  (if _output_get_2
    (Rendering|SetVisibility _laser true false)
    (bind _output_get_3 (Variables|Default|SetHitLocation (.Location (Collision|BreakHitResult _outhit))))
    (Effects|Components|ParticleSystem|SetVectorParameter _laser "LaserEnd" _output_get_3)))

(event EventBeginPlay
  ;[1 1 1] 레이저 색상 및
  (Rendering|SetVisibility (Variables|Default|GetLaser) false false)
  (Effects|Components|ParticleSystem|SetColorParameter (Variables|Default|GetLaser) "Color" "(R=0.165958,G=0.000000,B=0.812500,A=1.000000)")
  (Effects|Components|ParticleSystem|SetFloatParameter (Variables|Default|GetLaser) "LaserWidth" 2.0))

(event Collision|EventActorBeginOverlap
  (params (OtherActor :type Actor%20Object%20Reference)))

(event EventTick
  (params (DeltaSeconds :type Float%20%28single-precision%29))
  (bind _arrow (Variables|Default|GetArrow))
  ;[1 1 1] 미사일 생성
  (bind _output_get (Variables|Default|SetCurrentTime (+ DeltaSeconds (Variables|Default|GetCurrentTime))))
  (if (>= _output_get (Variables|Default|GetSpawnTime))
    (Game|SpawnActorfromClass "/Game/2_BP/BP_GlaDosTurretBullet.BP_GlaDosTurretBullet_C" (Math|Transform|MakeTransform (Transformation|GetWorldLocation _arrow) (Transformation|GetWorldRotation _arrow) "1.000000,1.000000,1.000000") "Undefined" "MultiplyWithRoot" 0 0)
    (Variables|Default|SetCurrentTime 0.0)))

(fn ConstructionScript)