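; BP_Laser is a red laser beam actor that can trigger a reflecting cube.
; Each Tick it line-traces between TraceVector's points, ending the Laser effect at the hit or maximum point and showing LaserImpact on blocking hits.
; It toggles ReflectionStart on the BP_Cube_Reflect found by GetActorOfClass, depending on whether that cube is hit.
; A player hit only performs a cast, with no further action.
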(event Collision|EventActorBeginOverlap
  (params (OtherActor :type Actor%20Object%20Reference)))

(event EventTick
  (params (DeltaSeconds :type Float%20%28single-precision%29))
  (bind _returnvalue (Game|GetPlayerCharacter 0))
  (bind (_returnvalue_2 _returnvalue2) (|TraceVector))
  (bind _laserimpact (Variables|Default|GetLaserImpact))
  (bind _output_get (Variables|Default|SetEndVector _returnvalue2))
  (bind _outhit (Collision|LineTraceByChannel _returnvalue_2 _output_get "TraceTypeQuery4" false 0 "None"))
  (Variables|Default|SetHit%20Bool (.bBlockingHit (Collision|BreakHitResult _outhit)))
  (Variables|Default|SetHit%20Location (.Location (Collision|BreakHitResult _outhit)))
  (Utilities|FlowControl|Sequence
    (:then_0
      (Effects|Components|ParticleSystem|SetVectorParameter (Variables|Default|GetLaser) "LaserEnd" (select (Variables|Default|GetHit%20Bool) (Variables|Default|GetHit%20Location) (Variables|Default|GetEndVector)))
      (Rendering|SetVisibility _laserimpact (Variables|Default|GetHit%20Bool) false)
      (Transformation|SetWorldLocation _laserimpact (Variables|Default|GetHit%20Location) false false))
    (:then_1
      (Utilities|FlowControl|Sequence
        (:then_0
          (if (== (.HitActor (Collision|BreakHitResult _outhit)) _returnvalue)
            (Utilities|Casting|CastToBP_SinglePlayer _returnvalue)))
        (:then_1
          (bind _returnvalue_3 (Actor|GetActorOfClass "/Game/2_BP/BP_Cube_Reflect.BP_Cube_Reflect_C"))
          (if (== (.HitActor (Collision|BreakHitResult _outhit)) _returnvalue_3)
            (Default|ReflectionStart _returnvalue_3 true)
            (else
              (Default|ReflectionStart _returnvalue_3 false))))))))

(event EventBeginPlay
  (bind _laser (Variables|Default|GetLaser))
  (Effects|Components|ParticleSystem|SetColorParameter _laser "Color" "(R=1.000000,G=0.000000,B=0.000000,A=1.000000)")
  (Effects|Components|ParticleSystem|SetFloatParameter _laser "LaserWidth" 4.0)
  (Effects|Components|ParticleSystem|SetColorParameter (Variables|Default|GetLaserImpact) "Color" "(R=1.000000,G=0.000000,B=0.000000,A=1.000000)"))

(fn ConstructionScript)