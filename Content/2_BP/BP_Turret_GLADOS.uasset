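; BP_Turret_GLADOS is a turret that tracks the player with a laser and fires missiles.
; When PawnSensing sees the player, it yaws toward them and line-traces forward from LaserPoint.
; A blocking hit of any kind shows the laser, sets its end point and calls Fire.
; Fire spawns BP_Turret_Missle after a SpawnTime Delay, which throttles repeated calls; the laser is never hidden again after BeginPlay.
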(event OnSeePawn(PawnSensing)
  (params (Pawn :type Pawn%20Object%20Reference))
  (bind _returnvalue (Transformation|GetActorLocation))
  (bind _returnvalue_2 (Game|GetPlayerCharacter 0))
  (if (== Pawn _returnvalue_2)
    (bind _asbp_single_player (Utilities|Casting|CastToBP_SinglePlayer _returnvalue_2))
    (bind _output_get (Variables|Default|SetWatchingRotation (Math|Rotator|FindLookatRotation (Math|Vector|MakeVector (.x _returnvalue) (.y _returnvalue) 0.0) (Math|Vector|MakeVector (.x (Transformation|GetActorLocation _asbp_single_player)) (.y (Transformation|GetActorLocation _asbp_single_player)) 0.0))))
    (Transformation|SetActorRotation _output_get)
    (CallFunction|LaserTrack)))

(event Custom|LaserTrack
  (bind _laser (Variables|Default|GetLaser))
  (bind _laserpoint (Variables|Default|GetLaserPoint))
  (bind _returnvalue (Transformation|GetWorldLocation _laserpoint))
  (bind _output_get (Variables|Default|SetEndVector (+ _returnvalue (* (Math|Vector|GetForwardVector _laserpoint) (Variables|Default|GetDistance)))))
  (bind _outhit (Collision|LineTraceByChannel _returnvalue _output_get "TraceTypeQuery1" false 0 "ForOneFrame"))
  (bind _output_get_2 (Variables|Default|SetHitBool (.bBlockingHit (Collision|BreakHitResult _outhit))))
  (if _output_get_2
    (Rendering|SetVisibility _laser true false)
    (bind _output_get_3 (Variables|Default|SetHitLocation (.Location (Collision|BreakHitResult _outhit))))
    (Effects|Components|ParticleSystem|SetVectorParameter _laser "LaserEnd" _output_get_3)
    (CallFunction|Fire)))

(event Custom|DitactPlayer)

(event Custom|Fire
  (Utilities|FlowControl|Delay (Variables|Default|GetSpawnTime))
  (Game|SpawnActorfromClass "/Game/2_BP/BP_Turret_Missle.BP_Turret_Missle_C" (Math|Transform|MakeTransform (Transformation|GetWorldLocation (Variables|Default|GetLaserPoint)) (Variables|Default|GetWatchingRotation) "1.000000,1.000000,1.000000") "Undefined" "MultiplyWithRoot" 0 0))

(event EventBeginPlay
  (bind _laser (Variables|Default|GetLaser))
  (Rendering|SetVisibility _laser false false)
  (Effects|Components|ParticleSystem|SetColorParameter _laser "Color" "(R=0.061908,G=0.020616,B=0.494792,A=1.000000)")
  (Effects|Components|ParticleSystem|SetFloatParameter _laser "LaserWidth" 2.0))

(event Collision|EventActorBeginOverlap
  (params (OtherActor :type Actor%20Object%20Reference)))

(event EventTick
  (params (DeltaSeconds :type Float%20%28single-precision%29)))

(fn ConstructionScript)