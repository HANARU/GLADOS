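; Portal gun component that lets the single-player character fire a blue or orange portal onto portal walls.
; On BeginPlay it attaches to the player's weapon socket, adds its Enhanced Input mapping context and hides itself from the owner.
; Left and right clicks trace from the first-person camera and ask the hit BP_PortalWall to place portal A or B.
; A successful placement destroys that slot's old portal and relinks the pair.
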(event Input|EnhancedActionEvents|EnhancedInputActionIA_MouseLeftClick
  (params (ActionValue :type Boolean) (ElapsedSeconds :type Float%20%28double-precision%29) (TriggeredSeconds :type Float%20%28double-precision%29) (InputAction :type Input%20Action%20Object%20Reference :default "/Game/4_MISC/Input/Action/IA_MouseLeftClick.IA_MouseLeftClick"))
  (bind _player (Variables|Default|GetPlayer))
  (bind _fpscam (Variables|/Script/GLADOS.SinglePlayer|GetFPSCAM _player))
  (:Started
    (CallFunction|SpawnPortalAlongVector (Transformation|GetWorldLocation _fpscam) (Math|Vector|GetForwardVector _fpscam) true)
    (Audio|PlaySound2D "/Game/3_Assets/Sound/SFX/BluePortal.BluePortal" 1.0 1.0 0.0 0 0)))

(event Input|EnhancedActionEvents|EnhancedInputActionIA_MouseRightClick
  (params (ActionValue :type Boolean) (ElapsedSeconds :type Float%20%28double-precision%29) (TriggeredSeconds :type Float%20%28double-precision%29) (InputAction :type Input%20Action%20Object%20Reference :default "/Game/4_MISC/Input/Action/IA_MouseRightClick.IA_MouseRightClick"))
  (bind _player (Variables|Default|GetPlayer))
  (bind _fpscam (Variables|/Script/GLADOS.SinglePlayer|GetFPSCAM _player))
  (:Started
    (CallFunction|SpawnPortalAlongVector (Transformation|GetWorldLocation _fpscam) (Math|Vector|GetForwardVector _fpscam) false)
    (Audio|PlaySound2D "/Game/3_Assets/Sound/SFX/OrangePortal.OrangePortal" 1.0 1.0 0.0 0 0)))

(event EventBeginPlay
  (bind _asbp_single_player (Utilities|Casting|CastToBP_SinglePlayer (Components|GetOwner)))
  (bind _output_get (Variables|Default|SetPlayer _asbp_single_player))
  (Transformation|AttachComponentToComponent (Variables|/Script/Engine.Character|GetMesh _output_get) "WeaponSocket" "SnapToTarget" "SnapToTarget" "SnapToTarget" true)
  (Default|HasGun (Variables|Default|GetPlayer))
  (bind _asplayer_controller (Utilities|Casting|CastToPlayerController (Pawn|GetController (Variables|Default|GetPlayer))))
  (Utilities|IsValid (PlayerController|LocalPlayerSubsystems|GetEnhancedInputLocalPlayerSubsystem _asplayer_controller)
    (:Is%20Valid
      (Input|AddMappingContext (PlayerController|LocalPlayerSubsystems|GetEnhancedInputLocalPlayerSubsystem _asplayer_controller) "/Game/4_MISC/Input/PortalGunMappingContext.PortalGunMappingContext" 1 "(bIgnoreAllPressedKeysUntilRelease=True,bForceImmediately=False)")
      (Class|PrimitiveComponent|SetOwnerNoSee true))))

(fn SpawnPortalAlongVector
  (params (StartLocation :type Vector) (Direction :type Vector) (PortalA :type Boolean))
  (bind _outhit (Collision|LineTraceForObjects StartLocation (+ StartLocation (* Direction (Variables|Default|GetMaxSpawnDistance))) (Utilities|Array|MakeArray "ObjectTypeQuery7") false 0 "None"))
  (bind _asbp_portal_wall (Utilities|Casting|CastToBP_PortalWall (.HitActor (Collision|BreakHitResult _outhit))))
  (bind _newportal (Default|TryAddPortal _asbp_portal_wall (+ (.Location (Collision|BreakHitResult _outhit)) (Math|Vector|Normalize (- (.TraceStart (Collision|BreakHitResult _outhit)) (.TraceEnd (Collision|BreakHitResult _outhit))))) PortalA))
  (bind _output_get (LocalVariables|SetNewPortal _newportal))
  (Utilities|IsValid _output_get
    (:Is%20Valid
      (CallFunction|SwapPortals (select PortalA (Variables|Default|GetPortalA) (Variables|Default|GetPortalB)) (LocalVariables|GetNewPortal))
      (Utilities|FlowControl|Sequence
        (:then_0
          (bind _portala (Variables|Default|GetPortalA)
            (:then
              (Default|LinkPortals _portala (Variables|Default|GetPortalB)))
            (:else)))
        (:then_1
          (bind _portalb (Variables|Default|GetPortalB)
            (:then
              (Default|LinkPortals _portalb (Variables|Default|GetPortalA)))
            (:else)))))))

(fn SwapPortals
  (params (OldPortal :type BP%20Portal%20Object%20Reference%20%28by%20ref%29) (NewPortal :type BP%20Portal%20Object%20Reference))
  (Utilities|FlowControl|Sequence
    (:then_0
      (Utilities|IsValid OldPortal
        (:Is%20Valid
          (Actor|DestroyActor OldPortal))))
    (:then_1
      (|SetBy-RefVar OldPortal NewPortal))))