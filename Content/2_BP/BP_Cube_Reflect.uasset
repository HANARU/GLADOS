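; Reflector cube that emits a red laser beam and impact effect when reflection is switched on.
; ReflectionStart traces from StartPoint along the player camera's forward vector with Z zeroed, so the beam follows the player's horizontal aim.
; The LaserCheck input, not the trace result, toggles both effects.
; The beam ends at the full trace distance, while the impact effect moves to the hit location.
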(event Custom|ReflectionStart
  (params (LaserCheck :type Boolean))
  (bind _laser (Variables|Default|GetLaser))
  (bind _laserimpact (Variables|Default|GetLaserImpact))
  (bind _laserimpact_2 (Variables|Default|GetLaserImpact))
  (bind _asbp_single_player (Utilities|Casting|CastToBP_SinglePlayer (Game|GetPlayerCharacter 0)))
  (bind _outhit (CallFunction|TrackingFront _asbp_single_player))
  (bind _output_get (Variables|Default|SetHit%20Bool LaserCheck))
  (Variables|Default|SetHit%20Location (.Location (Collision|BreakHitResult _outhit)))
  (if _output_get
    (Effects|Components|ParticleSystem|SetVectorParameter _laser "LaserEnd" (Variables|Default|GetEndVector))
    (Effects|Components|ParticleSystem|SetFloatParameter _laser "LaserWidth" 4.0)
    (Rendering|SetVisibility _laser (Variables|Default|GetHit%20Bool) false)
    (Rendering|SetVisibility _laserimpact (Variables|Default|GetHit%20Bool) false)
    (Transformation|SetWorldLocation _laserimpact (Variables|Default|GetHit%20Location) false false)
    (else
      (Effects|Components|ParticleSystem|SetVectorParameter _laser "LaserEnd" "0, 0, 0")
      (Rendering|SetVisibility _laser (Variables|Default|GetHit%20Bool) false)
      (Rendering|SetVisibility _laserimpact_2 (Variables|Default|GetHit%20Bool) false)
      (Transformation|SetWorldLocation _laserimpact_2 (Variables|Default|GetHit%20Location) false false))))

(event EventBeginPlay
  (bind _laser (Variables|Default|GetLaser))
  (bind _laserimpact (Variables|Default|GetLaserImpact))
  (Effects|Components|ParticleSystem|SetColorParameter _laser "Color" "(R=1.000000,G=0.000000,B=0.000000,A=1.000000)")
  (Rendering|SetVisibility _laser false false)
  (Effects|Components|ParticleSystem|SetColorParameter _laserimpact "Color" "(R=1.000000,G=0.000000,B=0.000000,A=1.000000)")
  (Rendering|SetVisibility _laserimpact false false))

(fn ConstructionScript)

(fn TrackingFront
  (params (Player :type Single%20Player%20Object%20Reference))
  (bind _startpoint (Variables|Default|GetStartPoint))
  (bind _fpscam (Variables|/Script/GLADOS.SinglePlayer|GetFPSCAM Player))
  (bind _distance (Variables|Default|GetDistance))
  (bind _returnvalue (Math|Vector|GetForwardVector _fpscam))
  (bind _returnvalue_2 (Transformation|GetWorldLocation _startpoint))
  (bind _returnvalue_3 (Math|Vector|MakeVector (.x _returnvalue) (.y _returnvalue) 0.0))
  (bind _returnvalue_4 (* _returnvalue_3 _distance))
  (bind _returnvalue_5 (+ _returnvalue_2 _returnvalue_4))
  (Variables|Default|SetEndVector _returnvalue_5)
  (bind (_outhit _returnvalue_6) (Collision|LineTraceByChannel _returnvalue_2 _returnvalue_5 "TraceTypeQuery5" false 0 "None"))
  (return _outhit _returnvalue_6))