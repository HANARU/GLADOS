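; BP_StandButton is an interactable stand button that lights up when the single-player character uses it nearby.
; Capsule overlaps with BP_SinglePlayer toggle an IsAble flag that gates the Interact event.
; Interact plays a timeline that drives the button material's Bright scalar and clears IsAble, so the player must re-enter the capsule to trigger it again.
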(event OnComponentBeginOverlap(Capsule)
  (params (OverlappedComponent :type Primitive%20Component%20Object%20Reference) (OtherActor :type Actor%20Object%20Reference) (OtherComp :type Primitive%20Component%20Object%20Reference) (OtherBodyIndex :type Integer) (bFromSweep :type Boolean) (SweepResult :type Hit%20Result%20Structure%20%28by%20ref%29))
  (Utilities|Casting|CastToBP_SinglePlayer OtherActor)
  (Variables|Default|SetbIsAble true))

(event OnComponentEndOverlap(Capsule)
  (params (OverlappedComponent :type Primitive%20Component%20Object%20Reference) (OtherActor :type Actor%20Object%20Reference) (OtherComp :type Primitive%20Component%20Object%20Reference) (OtherBodyIndex :type Integer))
  (Utilities|Casting|CastToBP_SinglePlayer OtherActor)
  (Variables|Default|SetbIsAble false))

(event EventInteract
  (if (Variables|Default|GetbIsAble)
    (bind _data (Timeline|Timeline PlayFromStart)
      (:Update
        (Rendering|Material|SetScalarParameterValueonMaterials (Variables|Default|GetButton) "Bright" (* _data 1e+02))
        (Variables|Default|SetbIsAble false)))))

(fn ConstructionScript)